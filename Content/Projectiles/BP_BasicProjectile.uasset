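; BP_BasicProjectile is a projectile that damages one designated target enemy.
; On BeginPlay it pushes its main collider along the actor's forward vector with a one-off AddForce, then destroys itself after a short delay in case it misses.
; Overlaps with anything other than TargetEnemy are ignored; hitting the target sends it a damage message with the Instigator and destroys the projectile.
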(event EventBeginPlay
  ;[1 1 1] Add force and destroy projectile if it missed
  (Physics|AddForce (Variables|Default|GetMainCollider) (* (Transformation|GetActorForwardVector) 7e+04) "None" false)
  (Utilities|FlowControl|Delay 3.0)
  (Actor|DestroyActor))

(event Collision|EventActorBeginOverlap
  (params (OtherActor :type Actor%20Object%20Reference))
  ;[1 1 1] Check for target on overlap
  (if (== OtherActor (Variables|Default|GetTargetEnemy))
    (Class|IKillable|ReceiveDamage(Message) OtherActor (Variables|Actor|GetInstigator))
    (Actor|DestroyActor)))

(fn ConstructionScript)