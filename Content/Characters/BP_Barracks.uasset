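; Barracks actor that spawns a unit near itself each time its Plane component is clicked, serving as either an enemy or a player barracks.
; The EnemyBarracks flag selects the enemy unit or a random short-, mid- or long-range player unit, and sets the text label in the Construction Script.
; Each unit spawns at a random navigable point around the barracks with a random yaw.
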(event OnClicked(Plane)
  (params (TouchedComponent :type Primitive%20Component%20Object%20Reference) (ButtonPressed :type Key%20Structure :default "None"))
  (Game|SpawnActorfromClass (select (Variables|Default|GetEnemyBarracks) "/Game/Characters/BP_EnemyUnit.BP_EnemyUnit_C" (Utilities|Select :Index (Math|Random|RandomIntegerinRange 0 2) :Option%200 "/Game/Characters/BP_PlayerUnit_ShortRange.BP_PlayerUnit_ShortRange_C" :Option%201 "/Game/Characters/BP_PlayerUnit_MidRange.BP_PlayerUnit_MidRange_C" :Option%202 "/Game/Characters/BP_PlayerUnit_LongRange.BP_PlayerUnit_LongRange_C")) (Math|Transform|MakeTransform (.RandomLocation (Class|NavigationSystemV1|GetRandomPointinNavigableRadius (Transformation|GetActorLocation) 2e+02 0 0)) (Math|Rotator|MakeRotator 0.0 0.0 (Math|Random|RandomFloatinRange 0.0 359.0)) "1,1,1") "Undefined" 0))

(fn ConstructionScript
  (Rendering|Components|TextRender|SetText (Variables|Default|GetTextRender) (select (Variables|Default|GetEnemyBarracks) (Utilities|Text|MakeLiteralText "Click to spawn enemy") (Utilities|Text|MakeLiteralText "Click to recruit units"))))