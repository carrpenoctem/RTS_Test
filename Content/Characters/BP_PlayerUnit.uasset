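; BP_PlayerUnit is a selectable RTS unit driven by the BT_PlayerAI behavior tree through blackboard keys.
; Selection tints the body via a dynamic material and updates the controller's SelectedUnits list.
; Perception locks the first sensed enemy unit while no valid Enemy is set, clearing TargetLocation; move orders are refused while that enemy is valid.
; Damage kills the unit immediately with an explosion effect.
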(event OnTargetPerceptionUpdated(AIPerception)
  (params (Actor :type Actor%20Object%20Reference) (Stimulus :type AI%20Stimulus%20Structure))
  (bind (_asbp_enemy_unit _bsuccess) (Utilities|Casting|CastToBP_EnemyUnit Actor))
  ;[1 0.6692 0.4223] Perception update
  (if (and _bsuccess (Utilities|Struct|BreakAIStimulus Stimulus))
    (CallFunction|TrySetEnemy _asbp_enemy_unit)))

(event Custom|TrySetEnemy
  (params (Unit :type RTS%20Unit%20Object%20Reference))
  (bind _returnvalue (Utilities|Name|MakeLiteralName "Enemy"))
  (bind _returnvalue_2 (AI|GetBlackboard 0))
  ;[1 0.817 0.3806] Set enemy
  (Utilities|IsValid (AI|Components|Blackboard|GetValueasObject _returnvalue_2 _returnvalue)
    (:Is%20Not%20Valid
      (AI|Components|Blackboard|SetValueasObject _returnvalue_2 _returnvalue Unit)
      (AI|Components|Blackboard|ClearValue _returnvalue_2 (Utilities|Name|MakeLiteralName "TargetLocation")))))

(event Custom|SetDestination
  (params (VectorValue :type Vector))
  (bind _returnvalue (AI|GetBlackboard 0))
  ;[1 0.817 0.3806] Set Destination
  (Utilities|IsValid (AI|Components|Blackboard|GetValueasObject _returnvalue (Utilities|Name|MakeLiteralName "Enemy"))
    (:Is%20Valid
      (Development|PrintString (Utilities|String|Append (Utilities|GetDisplayName self) " is busy fighting and can't move.")))
    (:Is%20Not%20Valid
      (AI|Components|Blackboard|SetValueasVector _returnvalue (Utilities|Name|MakeLiteralName "TargetLocation") VectorValue))))

(event EventBeginPlay
  (bind _body (Variables|Default|GetBody))
  ;[1 1 1] Begin Play
  (AI|RunBehaviorTree (AI|GetAIController self) "/Game/AI/BT_PlayerAI.BT_PlayerAI")
  (bind _returnvalue (Rendering|Material|CreateDynamicMaterialInstance _body 0 (Utilities|Array|Get(acopy) (Rendering|Material|GetMaterials _body)) "None" :!class /Script/Engine.PrimitiveComponent))
  (Variables|Default|SetDynMatInst _returnvalue)
  (AI|Components|Blackboard|SetValueasFloat (AI|GetBlackboard 0) (Utilities|Name|MakeLiteralName "AttackRange") (Variables|Default|GetAttackRange)))

(event EventDoDie
  ;[1 1 1] I_Killable functions
  (Effects|SpawnEmitteratLocation "/Game/StarterContent/Particles/P_Explosion.P_Explosion" (Transformation|GetActorLocation))
  (Actor|DestroyActor))

(event EventDamage
  (params (Instigator :type Actor%20Object%20Reference))
  ;[1 1 1] I_Killable functions
  (CallFunction|DoDie))

(event EventDoUnselect
  ;[1 1 1] Selection effect
  (Rendering|Material|SetVectorParameterValue (Variables|Default|GetDynMatInst) "Color" "(R=1.000000,G=1.000000,B=1.000000,A=1.000000)" :!class /Script/Engine.MaterialInstanceDynamic)
  (Utilities|Array|RemoveItem (Variables|/Game/Player/BP_RTS_Controller.BP_RTS_Controller_C|GetSelectedUnits (.AsBP%20RTS%20Controller (Utilities|Casting|CastToBP_RTS_Controller (Game|GetPlayerController 0)))) self))

(event EventDoSelect
  ;[1 1 1] Selection effect
  (Rendering|Material|SetVectorParameterValue (Variables|Default|GetDynMatInst) "Color" "(R=0.000000,G=1.000000,B=0.034785,A=1.000000)" :!class /Script/Engine.MaterialInstanceDynamic)
  (Utilities|Array|AddUnique (Variables|/Game/Player/BP_RTS_Controller.BP_RTS_Controller_C|GetSelectedUnits (.AsBP%20RTS%20Controller (Utilities|Casting|CastToBP_RTS_Controller (Game|GetPlayerController 0)))) self))

(fn ConstructionScript)