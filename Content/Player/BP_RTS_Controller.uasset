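; RTS player controller that handles unit selection, camera movement and move orders.
; Left mouse clears the selection and drives the HUD's selection drawing, while movement axes move the player pawn.
; Separate axes steer a single selected unit along world axes, blocked while its blackboard holds an Enemy.
; Command projects the cursor hit onto the navmesh and gives selected units destinations in a near-square grid formation for behavior-tree movement.
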(event Custom|UnselectAllUnits
  ;[1 1 1] Unit selection
  (bind _arrayelement (Utilities|Array|ReverseforEachLoop (Variables|Default|GetSelectedUnits))
    (:LoopBody
      (Class|ISelectable|DoUnselect(Message) _arrayelement))))

(event EventBeginPlay
  ;[1 1 1] Begin play
  (Variables|Default|SetbShowMouseCursor true)
  (Variables|Default|SetRTS_HUD (.AsRTS%20HUD (Utilities|Casting|CastToRTS_HUD (HUD|GetHUD)))))

(event Input|ActionEvents|InputActionCommand
  (params (Key :type Key%20Structure :default "None"))
  (bind _hitresult (Game|Player|GetHitResultUnderCursorbyChannel "TraceTypeQuery1" true))
  (bind _impactpoint (Collision|BreakHitResult _hitresult))
  (bind (_projectedlocation _returnvalue) (AI|Navigation|ProjectPointtoNavigation _impactpoint 0 0 "0, 0, 0"))
  ;[1 1 1] BT induced movement
  (:Pressed
    (if _returnvalue
      (Variables|Default|SetInitialLoc _projectedlocation)
      (for (_array_element _array_index) (Variables|Default|GetSelectedUnits)
        (Utilities|IsValid _array_element
          (:Is%20Valid
            (Default|SetDestination _array_element (CallFunction|CalculateFormation _array_index))))))))

(event Input|AxisEvents|InputAxisVerticalMove
  (params (AxisValue :type Float%20%28single-precision%29))
  (bind _returnvalue (Game|Player|GetPlayerPawn 0))
  ;[1 1 1] Camera movement
  (Pawn|Input|AddMovementInput _returnvalue (Transformation|GetActorForwardVector _returnvalue) AxisValue false))

(event Input|AxisEvents|InputAxisHorizontalMove
  (params (AxisValue :type Float%20%28single-precision%29))
  (bind _returnvalue (Game|Player|GetPlayerPawn 0))
  ;[1 1 1] Camera movement
  (Pawn|Input|AddMovementInput _returnvalue (Transformation|GetActorRightVector _returnvalue) AxisValue false))

(event Input|AxisEvents|InputAxisHorizontalMovePawn
  (params (AxisValue :type Float%20%28single-precision%29))
  (bind _selectedunits (Variables|Default|GetSelectedUnits))
  (bind _output (Utilities|Array|Get(acopy) _selectedunits))
  ;[1 1 1] Manual Unit movement
  (if (!= AxisValue 0.0)
    (if (== (Utilities|Array|Length _selectedunits) 1)
      (Utilities|IsValid (AI|Components|Blackboard|GetValueasObject (AI|GetBlackboard _output) (Utilities|Name|MakeLiteralName "Enemy"))
        (:Is%20Valid
          (Development|PrintString "Cannot move fighting unit"))
        (:Is%20Not%20Valid
          (Pawn|Input|AddMovementInput _output "0,1.000000, 0" AxisValue false)))
      (else
        (Development|PrintString "Select one unit for manual control")))))

(event Input|AxisEvents|InputAxisVerticalMovePawn
  (params (AxisValue :type Float%20%28single-precision%29))
  (bind _selectedunits (Variables|Default|GetSelectedUnits))
  (bind _output (Utilities|Array|Get(acopy) _selectedunits))
  ;[1 1 1] Manual Unit movement
  (if (!= AxisValue 0.0)
    (if (== (Utilities|Array|Length _selectedunits) 1)
      (Utilities|IsValid (AI|Components|Blackboard|GetValueasObject (AI|GetBlackboard _output) (Utilities|Name|MakeLiteralName "Enemy"))
        (:Is%20Valid
          (Development|PrintString "Cannot move fighting unit"))
        (:Is%20Not%20Valid
          (Pawn|Input|AddMovementInput _output "1.000000, 0, 0" AxisValue false)))
      (else
        (Development|PrintString "Select one unit for manual control")))))

(event Input|MouseEvents|LeftMouseButton
  (params (Key :type Key%20Structure :default "None"))
  (bind _rts_hud (Variables|Default|GetRTS_HUD))
  ;[1 1 1] Unit selection
  (:Pressed
    (CallFunction|UnselectAllUnits)
    (Default|DrawSelection _rts_hud))
  (:Released
    (Default|FinishSelection _rts_hud)))

(fn ConstructionScript)

(fn CalculateFormation
  (params (Index :type Integer))
  (bind _selectedunits (Variables|Default|GetSelectedUnits))
  (bind _initialloc (Variables|Default|GetInitialLoc))
  (bind _returnvalue (Utilities|Array|Length _selectedunits))
  (bind _returnvalue_2 (Math|Conversions|ToFloat(Integer) _returnvalue))
  (bind _returnvalue_3 (Math|Float|Sqrt _returnvalue_2))
  (bind _returnvalue_4 (Math|Float|Ceil _returnvalue_3))
  (return (Math|Vector|MakeVector (+ (.x _initialloc) (* (Math|Conversions|ToFloat(Integer) (Math|Integer|%(Integer) Index _returnvalue_4)) 1.2e+02)) (+ (.y _initialloc) (* (Math|Conversions|ToFloat(Integer) (/ Index _returnvalue_4)) 1.2e+02)) (.z _initialloc))))